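; AmmunitionBP is an ammo pickup that a TimeWarpCharacter collects by touching its collision sphere.
; Begin overlap destroys the actor and gathers all AmmunitionBP instances, whose count feeds only a disconnected debug print.
; End overlap increments CurrentAmmo, provided the TimeWarpCharacter also casts to FirstPersonCharacter.
; Other input-toggling and game mode cast nodes are unconnected and never run.
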(event OnComponentBeginOverlap(CollisionSphere)
  (params (OverlappedComponent :type Primitive%20Component%20Object%20Reference) (OtherActor :type Actor%20Object%20Reference) (OtherComp :type Primitive%20Component%20Object%20Reference) (OtherBodyIndex :type Integer) (bFromSweep :type Boolean) (SweepResult :type Hit%20Result%20Structure%20%28by%20ref%29))
  (Utilities|Casting|CastToTimeWarpCharacter OtherActor)
  (Actor|DestroyActor)
  (bind _outactors (Actor|GetAllActorsOfClass "AmmunitionBP_C")))

(event OnComponentEndOverlap(CollisionSphere)
  (params (OverlappedComponent :type Primitive%20Component%20Object%20Reference) (OtherActor :type Actor%20Object%20Reference) (OtherComp :type Primitive%20Component%20Object%20Reference) (OtherBodyIndex :type Integer))
  (bind _astime_warp_character (Utilities|Casting|CastToTimeWarpCharacter OtherActor))
  (bind _asfirst_person_character (Utilities|Casting|CastToFirstPersonCharacter _astime_warp_character))
  (Variables|/Script/TimeWarp.TimeWarpCharacter|SetCurrentAmmo _asfirst_person_character (+ (Variables|/Script/TimeWarp.TimeWarpCharacter|GetCurrentAmmo _asfirst_person_character) 1)))

(event EventBeginPlay)

(event Collision|EventActorBeginOverlap
  (params (OtherActor :type Actor%20Object%20Reference)))

(event EventTick
  (params (DeltaSeconds :type Float%20%28single-precision%29)))

(fn ConstructionScript)